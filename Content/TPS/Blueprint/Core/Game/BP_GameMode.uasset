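; BP_GameMode is the TPS game mode that handles player spawning, respawning and the win condition.
; Initial spawns use the Phase1 player start, while TryToRespawn asks BP_GameState whether respawn is allowed and restarts player 0 at the start tagged for the current phase.
; EnemyDead passes positive scores to BP_GameState and, when that returns true, shows the BPW_EndGame win screen with a mouse cursor.
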(fn ConstructionScript)

(fn TrytoRespawn
  (bind _returnvalue (Game|GetPlayerController 0))
  (bind _asbp_game_state (Utilities|Casting|CastToBP_GameState (Game|GetGameState)))
  (bind (_success _currentphase) (Default|CanPlayerRespawn _asbp_game_state))
  (if _success
    (Class|GameModeBase|RestartPlayeratPlayerStart _returnvalue (Class|GameModeBase|FindPlayerStart _returnvalue (Utilities|Select :Index _currentphase :Option%200 "Phase1" :Option%201 "Phase2" :Option%202 "Phase3" :Option%203 "Phase4" :Option%204 "Phase5")))
    (return true)
    (else
      (return _success))))

(fn ChoosePlayerStart
  (params (Player :type Controller%20Object%20Reference))
  (return (Class|GameModeBase|FindPlayerStart Player "Phase1")))

(fn EnemyDead
  (params (Score :type Integer))
  (if (> Score 0)
    (bind _asbp_game_state (Utilities|Casting|CastToBP_GameState (Game|GetGameState)))
    (bind _biswin (Default|IncrementScore _asbp_game_state Score))
    (if _biswin
      (bind _returnvalue (UserInterface|CreateWidget "/Game/TPS/Blueprint/Widget/BPW_EndGame.BPW_EndGame_C" 0 true))
      (UserInterface|Viewport|AddtoViewport _returnvalue 0)
      (Variables|/Script/Engine.PlayerController|SetbShowMouseCursor (Game|GetPlayerController 0) true))))