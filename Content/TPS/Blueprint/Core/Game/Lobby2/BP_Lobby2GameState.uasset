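; Lobby game state that maintains the list of player states and keeps the local lobby menu's player list up to date.
; Adding or removing a player state, the PlayersList OnRep and the OnPlayerDataChanged event all trigger a refresh.
; The refresh casts player controller 0 to BP_Lobby2PlayerController and passes the list to its LobbyMenu, doing nothing if the cast fails.
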(event Custom|OnPlayerDataChanged
  (CallFunction|RefreshPlayerList))

(event EventTick
  (params (DeltaSeconds :type Float%20%28single-precision%29)))

(fn ConstructionScript)

(fn OnRepPlayersList
  (CallFunction|RefreshPlayerList))

(fn RefreshPlayerList
  (bind _asbp_lobby_2player_controller (Utilities|Casting|CastToBP_Lobby2PlayerController (Game|GetPlayerController 0)))
  (Default|RefreshPlayersList (Variables|/Game/TPS/Blueprint/Core/Game/Lobby2/BP_Lobby2PlayerController.BP_Lobby2PlayerController_C|GetLobbyMenu _asbp_lobby_2player_controller) (Variables|Default|GetPlayersList)))

(fn AddPlayerState
  (params (PlayerState :type Player%20State%20Object%20Reference))
  (Utilities|Array|Add (Variables|Default|GetPlayersList) PlayerState)
  (CallFunction|RefreshPlayerList))

(fn RemovePlayerState
  (params (PlayerState :type Player%20State%20Object%20Reference))
  (Utilities|Array|RemoveItem (Variables|Default|GetPlayersList) PlayerState)
  (CallFunction|RefreshPlayerList))