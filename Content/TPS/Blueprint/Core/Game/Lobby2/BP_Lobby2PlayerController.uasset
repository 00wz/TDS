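; BP_Lobby2PlayerController is the player controller for the Lobby2 screen, with the mouse cursor shown from BeginPlay.
; OnSelfPostLogin creates the BPW_LobbyMenu2 widget, adds it to the viewport and fills in the player's name.
; ChangeName forwards name changes to BP_LobbyMode2 through the game mode, passing itself as the controller.
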(event Custom|OnSelfPostLogin
  (params (SelfName :type String))
  (bind _returnvalue (UserInterface|CreateWidget "/Game/TPS/Blueprint/Widget/Menu/LobbyMenu/BPW_LobbyMenu2.BPW_LobbyMenu2_C"))
  (bind _output_get (Variables|Default|SetLobbyMenu _returnvalue))
  (UserInterface|Viewport|AddtoViewport _output_get 0)
  (Default|RefreshPlayerName (Variables|Default|GetLobbyMenu) (Utilities|Text|ToText(String) SelfName)))

(event Custom|ChangeName
  (params (NewName :type String))
  (bind _asbp_lobby_mode_2 (Utilities|Casting|CastToBP_LobbyMode2 (Game|GetGameMode)))
  (Default|ChangePlayerName _asbp_lobby_mode_2 self NewName))

(event EventBeginPlay
  (Variables|Default|SetbShowMouseCursor true))

(event EventTick
  (params (DeltaSeconds :type Float%20%28single-precision%29)))

(fn ConstructionScript)