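; Game mode for the Lobby2 multiplayer lobby that keeps the game state's player list in step with who is connected.
; On login it passes the player's name to their BP_Lobby2PlayerController and adds their PlayerState to BP_Lobby2GameState.
; On logout it removes that PlayerState.
; ChangePlayerName renames a controller's player through ChangeName, then notifies the game state of the change.
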(event EventBeginPlay)

(event EventTick
  (params (DeltaSeconds :type Float%20%28single-precision%29)))

(event EventPostLogin
  (params (NewPlayer :type Player%20Controller%20Object%20Reference))
  (bind _playerstate (Variables|/Script/Engine.Controller|GetPlayerState NewPlayer))
  (bind _asbp_lobby_2player_controller (Utilities|Casting|CastToBP_Lobby2PlayerController NewPlayer))
  (Default|OnSelfPostLogin _asbp_lobby_2player_controller (PlayerState|GetPlayerName _playerstate))
  (bind _asbp_lobby_2game_state (Utilities|Casting|CastToBP_Lobby2GameState (Game|GetGameState)))
  (Default|AddPlayerState _asbp_lobby_2game_state _playerstate))

(event EventOnLogout
  (params (ExitingController :type Controller%20Object%20Reference))
  (bind _asbp_lobby_2game_state (Utilities|Casting|CastToBP_Lobby2GameState (Game|GetGameState)))
  (Default|RemovePlayerState _asbp_lobby_2game_state (Variables|/Script/Engine.Controller|GetPlayerState ExitingController)))

(fn ConstructionScript)

(fn ChangePlayerName
  (params (Controller :type Player%20Controller%20Object%20Reference) (NewName :type String))
  (Class|GameModeBase|ChangeName Controller NewName true)
  (bind _asbp_lobby_2game_state (Utilities|Casting|CastToBP_Lobby2GameState (Game|GetGameState)))
  (Default|OnPlayerNameChanged _asbp_lobby_2game_state))