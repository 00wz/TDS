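; Player controller for the multiplayer lobby, linking each player's menu, lobby character and BP_LobbyMode.
; On BeginPlay it views the first CameraActor found and gives the local player a lobby menu that knows whether they host.
; Color and map choices go to the game mode, menu updates come back through client events, and ready, animation and color changes forward to the saved character.
; The authority destroys that character with the controller.
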(event Custom|SaveLobbyCharacter
  (params (LobbyCharacter :type BP%20Lobby%20Character%20Object%20Reference))
  (Variables|Default|SetLobbyCharacter LobbyCharacter))

(event Custom|UdpateLobbyCharacterParam
  (params (Material :type Material%20Interface%20Object%20Reference))
  (Default|ChangeColoronServer (Variables|Default|GetLobbyCharacter) Material))

(event Custom|UpdateMeReady
  (Default|MeReadyMulticast (Variables|Default|GetLobbyCharacter)))

(event Custom|UpdatePlayerSelectMap
  (params (LevelName :type Name))
  (bind _asbp_lobby_mode (Utilities|Casting|CastToBP_LobbyMode (Game|GetGameMode)))
  (Default|UpdateLevelName _asbp_lobby_mode LevelName))

(event Custom|UpdateLobbyWidget_OnClient
  (params (Name :type Name))
  (Default|UpdateLevelName (Variables|Default|GetLobbyWidget) Name))

(event Custom|RemoveAllWidget
  (Viewport|RemoveAllWidgets))

(event Custom|SelectedNewColor
  (params (NewColor :type Material%20Interface%20Object%20Reference))
  (bind _asbp_lobby_mode (Utilities|Casting|CastToBP_LobbyMode (Game|GetGameMode)))
  (Default|UpdateColorforCharacter _asbp_lobby_mode NewColor self))

(event Custom|UpdateColorsLobbyWidget_OnClient
  (params (Blocks :type Array%20of%20Material%20Interface%20Object%20References))
  (bind _lobbywidget (Variables|Default|GetLobbyWidget))
  (Utilities|IsValid _lobbywidget
    (:Is%20Valid
      (Default|UpdateAviableColors _lobbywidget Blocks))))

(event Custom|PlayAnimOnServer
  (Default|PlayAnimMulticast (Variables|Default|GetLobbyCharacter)))

(event EventBeginPlay
  (bind _returnvalue (Networking|IsServer))
  (Variables|Default|SetbShowMouseCursor true)
  (bind _outactors (Actor|GetAllActorsOfClass "/Script/Engine.CameraActor"))
  (Game|Player|SetViewTargetwithBlend (Utilities|Array|Get(acopy) _outactors) 0.0 "VTBlend_Linear" 0.0 false)
  (if (Pawn|IsLocalPlayerController)
    (bind _returnvalue_2 (UserInterface|CreateWidget "/Game/TPS/Blueprint/Widget/Menu/LobbyMenu/BPW_LobbyMenu.BPW_LobbyMenu_C" 0 _returnvalue))
    (bind _output_get (Variables|Default|SetLobbyWidget _returnvalue_2))
    (UserInterface|Viewport|AddtoViewport _returnvalue_2 0)
    (if (not _returnvalue)
      (Default|UpdateLevelName _output_get (Variables|Default|GetCurrentLevelByServer)))))

(event EventDestroyed
  (Networking|SwitchHasAuthority
    (:Authority
      (Actor|DestroyActor (Variables|Default|GetLobbyCharacter)))))

(event Input|KeyboardEvents|T
  (params (Key :type Key%20Structure :default "None"))
  (:Pressed
    (CallFunction|PlayAnimonServer)))

(fn ConstructionScript)