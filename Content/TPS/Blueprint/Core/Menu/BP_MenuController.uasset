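; BP_MenuController is the player controller for the menu, creating and switching between the main menu and multiplayer menu widgets.
; On BeginPlay, for the local controller only, it adds both widgets to the viewport, shows the main menu and enables the mouse cursor.
; ShowMainMenu and ShowMultiplayerMenu toggle the two widgets between Visible and Collapsed, so both persist rather than being recreated on each switch.
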(event EventBeginPlay
  (bind _returnvalue (Game|GetPlayerController 0))
  (if (Pawn|IsLocalPlayerController)
    (bind _returnvalue_2 (UserInterface|CreateWidget "/Game/TPS/Blueprint/Widget/Menu/BPW_Menu.BPW_Menu_C" _returnvalue))
    (UserInterface|Viewport|AddtoViewport _returnvalue_2 0)
    (Variables|Default|SetMainMenu _returnvalue_2)
    (bind _returnvalue_3 (UserInterface|CreateWidget "/Game/TPS/Blueprint/Widget/Menu/BPW_MultiplayerMenu.BPW_MultiplayerMenu_C" _returnvalue))
    (UserInterface|Viewport|AddtoViewport _returnvalue_3 0)
    (Variables|Default|SetMultiplayerMenu _returnvalue_3)
    (CallFunction|ShowMainMenu)
    (Variables|/Script/Engine.PlayerController|SetbShowMouseCursor _returnvalue true)))

(fn ConstructionScript)

(fn ShowMainMenu
  (Widget|SetVisibility (Variables|Default|GetMainMenu) "Visible")
  (Widget|SetVisibility (Variables|Default|GetMultiplayerMenu) "Collapsed"))

(fn ShowMultiplayerMenu
  (Widget|SetVisibility (Variables|Default|GetMainMenu) "Collapsed")
  (Widget|SetVisibility (Variables|Default|GetMultiplayerMenu) "Visible"))