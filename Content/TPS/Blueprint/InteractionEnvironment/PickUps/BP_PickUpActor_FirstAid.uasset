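; First-aid pickup actor that restores health to a character who overlaps it.
; It extends the parent pickup's OverlapCharacter event, finding the BP_Character through the owner of the passed inventory.
; If that character's health component reads below a hard-coded 100, it applies Value through ChangeHealthValueOnServer and calls PickUpSuccess.
; At or above that threshold, this child neither heals nor reports a successful pickup.
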(event EventBeginPlay
  (|CallParentFunction) ; This node is disabled and will not be called.\nDrag off pins to build functionality.
)

(event Collision|EventActorBeginOverlap
  (params (OtherActor :type Actor%20Object%20Reference))
  (|CallParentFunction OtherActor) ; This node is disabled and will not be called.\nDrag off pins to build functionality.
)

(event EventTick
  (params (DeltaSeconds :type Float%20%28single-precision%29))
  (|CallParentFunction DeltaSeconds) ; This node is disabled and will not be called.\nDrag off pins to build functionality.
)

(event EventOverlapCharacter
  (params (ToInventory :type TPS%20Inventory%20Component%20Object%20Reference))
  (|CallParentFunction ToInventory)
  (bind _asbp_character (Utilities|Casting|CastToBP_Character (Components|GetOwner ToInventory)))
  (bind _returnvalue (Class|TPSHealthComponent|GetCurrentHealth (Variables|/Script/TPS.TPSCharacter|GetCharHealthComponent _asbp_character)))
  (if (< _returnvalue 1e+02)
    (Class|TPSHealthComponent|ChangeHealthValueonServer (Variables|/Script/TPS.TPSCharacter|GetCharHealthComponent _asbp_character) (Variables|Default|GetValue))
    (CallFunction|PickUpSuccess)))

(fn ConstructionScript
  (|CallParentFunction))