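; Ammo pickup actor for the TPS game that gives ammo of a selected weapon type to an overlapping character's inventory.
; On BeginPlay, InitActor uses the weapon type to select the static mesh and spinner particle, destroying either component if its asset is invalid.
; The parent's OverlapCharacter event is extended to check that the inventory can take that ammo, add the configured count and trigger pickup success.
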(event EventBeginPlay
  (|CallParentFunction)
  (CallFunction|InitActor))

(event Collision|EventActorBeginOverlap
  (params (OtherActor :type Actor%20Object%20Reference))
  (|CallParentFunction OtherActor) ; This node is disabled and will not be called.\nDrag off pins to build functionality.
)

(event EventTick
  (params (DeltaSeconds :type Float%20%28single-precision%29))
  (|CallParentFunction DeltaSeconds) ; This node is disabled and will not be called.\nDrag off pins to build functionality.
)

(event EventOverlapCharacter
  (params (ToInventory :type TPS%20Inventory%20Component%20Object%20Reference))
  (bind _weapontypeammo (Variables|Default|GetWeaponTypeAmmo))
  (|CallParentFunction ToInventory)
  (bind _returnvalue (Class|TPSInventoryComponent|CheckCanTakeAmmo ToInventory _weapontypeammo))
  (if _returnvalue
    (Class|TPSInventoryComponent|AmmoSlotChangeValue ToInventory _weapontypeammo (Variables|Default|GetCout))
    (CallFunction|PickUpSuccess)))

(fn ConstructionScript
  (|CallParentFunction))

(fn InitActor
  (bind _weapontypeammo (Variables|Default|GetWeaponTypeAmmo))
  (bind _staticmesh (Variables|Default|GetStaticMesh))
  (bind _particlesystem (Variables|Default|GetParticleSystem))
  (bind _returnvalue (Utilities|Select :Index _weapontypeammo :RifleType "/Game/TPS/Effect/FX_PickUpActor/FX_Monsters/FX_Monster_Elemental/ICE/P_Spinner_Ammo_Rifle.P_Spinner_Ammo_Rifle" :ShotGunType "/Game/TPS/Effect/FX_PickUpActor/FX_Monsters/FX_Monster_Elemental/ICE/P_Spinner_Ammo_ShotGun.P_Spinner_Ammo_ShotGun" :SniperRifle "/Game/TPS/Effect/FX_PickUpActor/FX_Monsters/FX_Monster_Elemental/ICE/P_Spinner_Ammo_SniperRifle.P_Spinner_Ammo_SniperRifle" :GrenadeLauncher "/Game/TPS/Effect/FX_PickUpActor/FX_Monsters/FX_Monster_Elemental/ICE/P_Spinner_Ammo_Grenade.P_Spinner_Ammo_Grenade" :RocketLauncher "/Game/TPS/Effect/FX_PickUpActor/FX_Monsters/FX_Monster_Elemental/ICE/P_Spinner_Ammo_Rockets.P_Spinner_Ammo_Rockets"))
  (bind _returnvalue_2 (Utilities|Select :Index _weapontypeammo :RifleType "/Game/TPS/Items/GameActor/Weapon/Weapon_Rifle/Darkness_AssaultRifle_Pickup.Darkness_AssaultRifle_Pickup" :ShotGunType "/Game/TPS/Items/GameActor/Weapon/Weapon_ShotGun/Darkness_Shotgun_Pickup.Darkness_Shotgun_Pickup" :SniperRifle "/Game/TPS/Items/GameActor/Weapon/Weapon_SniperRifle/Darkness_SniperRifle_Pickup.Darkness_SniperRifle_Pickup" :GrenadeLauncher "/Game/TPS/Items/GameActor/Weapon/Weapon_GrenadeLauncher/Darkness_GrenadeLauncher_Pickup.Darkness_GrenadeLauncher_Pickup" :RocketLauncher "/Game/TPS/Items/GameActor/Weapon/Weapon_RocketLauncher/Darkness_RocketLauncher_Pickup.Darkness_RocketLauncher_Pickup"))
  (Utilities|FlowControl|Sequence
    (:then_0
      (Utilities|IsValid _returnvalue_2
        (:Is%20Valid
          (Components|StaticMesh|SetStaticMesh _staticmesh _returnvalue_2)
          (Transformation|SetRelativeLocation _staticmesh "0, 0, 0" false false)
          (Transformation|SetRelativeScale3D _staticmesh "2.000000,2.000000,2.000000")
          (Transformation|SetRelativeRotation _staticmesh (Math|Rotator|MakeRotator 0.0 0.0 0.0) false false))
        (:Is%20Not%20Valid
          (Components|DestroyComponent _staticmesh))))
    (:then_1
      (Utilities|IsValid _returnvalue
        (:Is%20Valid
          (Effects|Components|ParticleSystem|SetTemplate _particlesystem _returnvalue)
          (Transformation|SetRelativeScale3D _particlesystem "1.000000,1.000000,1.000000"))
        (:Is%20Not%20Valid
          (Components|DestroyComponent _particlesystem))))))