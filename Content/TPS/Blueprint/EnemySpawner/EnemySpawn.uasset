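; Enemy spawn point that registers itself with BP_GameMode at BeginPlay under its assigned phase.
; It converts its Phase value to a string and takes the first numeric character as the phase index.
; That index selects one of five per-phase spawn point arrays on the game mode, with index 0 mapping to Phase1, and the actor adds itself to it.
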(event EventBeginPlay
  (CallFunction|NewFunction0))

(fn ConstructionScript)

(fn NewFunction0
  (bind _array_element (Utilities|Array|ForEachLoopwithBreak (Utilities|String|GetCharacterArrayfromString (Utilities|String|ToString(Name) (Variables|Default|GetPhase))) :!label _label)
    (:LoopBody
      (if (Class|KismetStringLibrary|IsNumeric _array_element)
        (LocalVariables|SetCurrentPhasePoint (Math|Conversions|ToInteger(Byte) _array_element))
        (goto _label Break)))
    (:Completed
      (bind _asbp_game_mode (Utilities|Casting|CastToBP_GameMode (Game|GetGameMode)))
      (Utilities|Array|Add (Utilities|Select :Index (LocalVariables|GetCurrentPhasePoint) :Option%200 (Variables|/Game/TPS/Blueprint/Core/Game/BP_GameMode.BP_GameMode_C|GetSpawnPointPhase1 _asbp_game_mode) :Option%201 (Variables|/Game/TPS/Blueprint/Core/Game/BP_GameMode.BP_GameMode_C|GetSpawnPointPhase2 _asbp_game_mode) :Option%202 (Variables|/Game/TPS/Blueprint/Core/Game/BP_GameMode.BP_GameMode_C|GetSpawnPointPhase3 _asbp_game_mode) :Option%203 (Variables|/Game/TPS/Blueprint/Core/Game/BP_GameMode.BP_GameMode_C|GetSpawnPointPhase4 _asbp_game_mode) :Option%204 (Variables|/Game/TPS/Blueprint/Core/Game/BP_GameMode.BP_GameMode_C|GetSpawnPointPhase5 _asbp_game_mode)) self))))