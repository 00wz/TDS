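; Door actor that slides vertically when a Character enters its open trigger and returns when one enters its close trigger.
; Separate overlap volumes call Opening and Closing, which use an IsOpen flag to ignore repeat requests.
; One timeline drives the DoorRoot relative Z offset, playing forward to open and in reverse to close.
; An explosion sound cue plays at the actor's location whenever the timeline finishes.
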(event OnComponentBeginOverlap(OpenTrigger)
  (params (OverlappedComponent :type Primitive%20Component%20Object%20Reference) (OtherActor :type Actor%20Object%20Reference) (OtherComp :type Primitive%20Component%20Object%20Reference) (OtherBodyIndex :type Integer) (bFromSweep :type Boolean) (SweepResult :type Hit%20Result%20Structure%20%28by%20ref%29))
  (Utilities|Casting|CastToCharacter OtherActor)
  (CallFunction|Opening))

(event OnComponentBeginOverlap(CloseTrigger)
  (params (OverlappedComponent :type Primitive%20Component%20Object%20Reference) (OtherActor :type Actor%20Object%20Reference) (OtherComp :type Primitive%20Component%20Object%20Reference) (OtherBodyIndex :type Integer) (bFromSweep :type Boolean) (SweepResult :type Hit%20Result%20Structure%20%28by%20ref%29))
  (Utilities|Casting|CastToCharacter OtherActor)
  (CallFunction|Closing))

(event Custom|Opening
  (if (not (Variables|Default|GetIsOpen))
    (Variables|Default|SetIsOpen true)
    (bind _zoffset (Timeline|OpeningTimeline Play)
      (:Update
        (Transformation|SetRelativeLocation (Variables|Default|GetDoorRoot) (Math|Vector|MakeVector 0.0 0.0 _zoffset) false false))
      (:Finished
        (Audio|PlaySoundatLocation "/Game/StarterContent/Audio/Explosion_Cue.Explosion_Cue" (Transformation|GetActorLocation) "0, 0, 0" 1.0 1.0 0.0 0 0 0)))))

(event Custom|Closing
  (if (Variables|Default|GetIsOpen)
    (Variables|Default|SetIsOpen false)
    (bind _zoffset (Timeline|OpeningTimeline Reverse)
      (:Update
        (Transformation|SetRelativeLocation (Variables|Default|GetDoorRoot) (Math|Vector|MakeVector 0.0 0.0 _zoffset) false false))
      (:Finished
        (Audio|PlaySoundatLocation "/Game/StarterContent/Audio/Explosion_Cue.Explosion_Cue" (Transformation|GetActorLocation) "0, 0, 0" 1.0 1.0 0.0 0 0 0)))))

(event EventBeginPlay)

(event Collision|EventActorBeginOverlap
  (params (OtherActor :type Actor%20Object%20Reference)))

(event EventTick
  (params (DeltaSeconds :type Float%20%28single-precision%29)))

(fn ConstructionScript)