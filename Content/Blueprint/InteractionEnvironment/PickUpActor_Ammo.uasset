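; Ammo pickup actor that adds ammo to a character's inventory on overlap.
; It extends a parent pickup by overriding OverlapCharacter to ask the inventory whether it can take its weapon ammo type.
; If it can, it changes that ammo slot by the pickup's count and calls PickUpSuccess.
; Construction and InitActor overrides only call their parent versions.
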(event EventBeginPlay
  (|CallParentFunction) ; This node is disabled and will not be called.\nDrag off pins to build functionality.
)

(event Collision|EventActorBeginOverlap
  (params (OtherActor :type Actor%20Object%20Reference))
  (|CallParentFunction OtherActor) ; This node is disabled and will not be called.\nDrag off pins to build functionality.
)

(event EventTick
  (params (DeltaSeconds :type Float%20%28single-precision%29))
  (|CallParentFunction DeltaSeconds) ; This node is disabled and will not be called.\nDrag off pins to build functionality.
)

(event EventOverlapCharacter
  (params (ToInventory :type TPS%20Inventory%20Component%20Object%20Reference))
  (bind _weapontypeammo (Variables|Default|GetWeaponTypeAmmo))
  (|CallParentFunction ToInventory)
  (bind _returnvalue (Class|TPSInventoryComponent|CheckCanTakeAmmo ToInventory _weapontypeammo))
  (if _returnvalue
    (Class|TPSInventoryComponent|AmmoSlotChangeValue ToInventory _weapontypeammo (Variables|Default|GetCout))
    (CallFunction|PickUpSuccess)))

(fn ConstructionScript
  (|CallParentFunction))

(fn InitActor
  (params (InfoActor :type Drop%20Item%20Structure))
  (|CallParentFunction ""))