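; Base destructible environment actor that takes damage through a TPSHealth component and explodes when its health runs out.
; AnyDamage passes the negated damage to TPSHealth, whose health-change event spawns a DisplayDamageActor at a randomly jittered offset to show damage and current health.
; On death, the DestroyActor function removes the actor and spawns an explosion sound and particle effect at its location.
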(event OnHealthChange(TPSHealth)
  (params (Health :type Float%20%28single-precision%29) (Damage :type Float%20%28single-precision%29))
  (bind _returnvalue (Game|SpawnActorfromClass "/Game/Blueprint/InteractionEnvironment/DisplayDamage/DisplayDamageActor.DisplayDamageActor_C" (Math|Transform|MakeTransform (+ (+ (Math|Vector|MakeVector (Math|Random|RandomFloatinRange -2e+01 2e+01) (Math|Random|RandomFloatinRange -2e+01 2e+01) 0.0) (Variables|Default|GetLocalPointSpawnHealthNumber)) (Transformation|GetActorLocation))) "AlwaysSpawn" 0 0))
  (Default|InitActor _returnvalue Damage Health))

(event OnDead(TPSHealth)
  (CallFunction|DestroyActor))

(event EventBeginPlay)

(event Game|Damage|EventAnyDamage
  (params (Damage :type Float%20%28single-precision%29) (DamageType :type Damage%20Type%20Object%20Reference) (InstigatedBy :type Controller%20Object%20Reference) (DamageCauser :type Actor%20Object%20Reference))
  (Class|TPSHealthComponent|ChangeHealthValue (Variables|Default|GetTPSHealth) (* Damage -1.0)))

(event Game|Damage|EventRadialDamage
  (params (DamageReceived :type Float%20%28single-precision%29) (DamageType :type Damage%20Type%20Object%20Reference) (Origin :type Vector :default "0, 0, 0") (HitInfo :type Hit%20Result%20Structure%20%28by%20ref%29) (InstigatedBy :type Controller%20Object%20Reference) (DamageCauser :type Actor%20Object%20Reference)))

(event Game|Damage|EventPointDamage
  (params (Damage :type Float%20%28single-precision%29) (DamageType :type Damage%20Type%20Object%20Reference) (HitLocation :type Vector :default "0, 0, 0") (HitNormal :type Vector :default "0, 0, 0") (HitComponent :type Primitive%20Component%20Object%20Reference) (BoneName :type Name :default "None") (ShotFromDirection :type Vector :default "0, 0, 0") (InstigatedBy :type Controller%20Object%20Reference) (DamageCauser :type Actor%20Object%20Reference) (HitInfo :type Hit%20Result%20Structure%20%28by%20ref%29)))

(fn ConstructionScript)

(fn DestroyActor
  (bind _returnvalue (Transformation|GetActorLocation))
  (Actor|DestroyActor)
  (Audio|SpawnSoundatLocation "/Game/Fx_Effect/Sound/Explosion_Cue.Explosion_Cue" _returnvalue "0, 0, 0" 1.0 1.0 0.0 0 0)
  (Effects|SpawnEmitteratLocation "/Game/Fx_Effect/Particles/TPS_P_Explosion.TPS_P_Explosion" _returnvalue))