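; Weapon pickup actor, a child of a base pickup, that gives its WeaponInfo to the inventory of an overlapping character.
; InitActor stores the WeaponInfo before calling the parent initialization.
; On overlap it calls TryGetWeaponToInventory, finishing with PickUpSuccess or, on failure, starting a weapon switch on the owning BP_Character with itself as candidate.
; Leaving the Sphere ends that character's weapon switch.
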(event OnComponentEndOverlap(Sphere)
  (params (OverlappedComponent :type Primitive%20Component%20Object%20Reference) (OtherActor :type Actor%20Object%20Reference) (OtherComp :type Primitive%20Component%20Object%20Reference) (OtherBodyIndex :type Integer))
  (bind _asbp_character (Utilities|Casting|CastToBP_Character OtherActor))
  (Default|EndSwithcWeapon _asbp_character))

(event EventBeginPlay
  (|CallParentFunction) ; This node is disabled and will not be called.\nDrag off pins to build functionality.
)

(event Collision|EventActorBeginOverlap
  (params (OtherActor :type Actor%20Object%20Reference))
  (|CallParentFunction OtherActor) ; This node is disabled and will not be called.\nDrag off pins to build functionality.
)

(event EventTick
  (params (DeltaSeconds :type Float%20%28single-precision%29))
  (|CallParentFunction DeltaSeconds) ; This node is disabled and will not be called.\nDrag off pins to build functionality.
)

(event EventOverlapCharacter
  (params (ToInventory :type TPS%20Inventory%20Component%20Object%20Reference))
  (|CallParentFunction ToInventory)
  (bind _returnvalue (Class|TPSInventoryComponent|TryGetWeapontoInventory ToInventory (Variables|Default|GetWeaponInfo)))
  (if _returnvalue
    (CallFunction|PickUpSuccess)
    (else
      (bind _asbp_character (Utilities|Casting|CastToBP_Character (Components|GetOwner ToInventory)))
      (Default|StartSwithcWeapon _asbp_character self))))

(fn ConstructionScript
  (|CallParentFunction))

(fn InitActor
  (params (InfoActor :type Drop%20Item%20Structure))
  (Variables|Default|SetWeaponInfo (.WeaponInfo (Utilities|Struct|BreakDropItem InfoActor)))
  (|CallParentFunction InfoActor))